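; BP_Pickup is a drivable vehicle pawn that maps movement axes to throttle and steering, and look axes to controller pitch and yaw.
; A Box overlap calls CallCanDive on begin and CallCanWalk on end.
; Jump at near standstill teleports the vehicle slightly upward, keeping only its yaw, to right it.
; The construction script hides Sunny and several Item components in game; handbrake calls are unwired.
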(event OnComponentBeginOverlap(Box)
  (params (OverlappedComponent :type Primitive%20Component%20Object%20Reference) (OtherActor :type Actor%20Object%20Reference) (OtherComp :type Primitive%20Component%20Object%20Reference) (OtherBodyIndex :type Integer) (bFromSweep :type Boolean) (SweepResult :type Hit%20Result%20Structure%20%28by%20ref%29))
  (Default|CallCanDive))

(event OnComponentEndOverlap(Box)
  (params (OverlappedComponent :type Primitive%20Component%20Object%20Reference) (OtherActor :type Actor%20Object%20Reference) (OtherComp :type Primitive%20Component%20Object%20Reference) (OtherBodyIndex :type Integer))
  (Default|CallCanWalk))

(event Custom|Upright%20Vehicle
  (bind _mesh (Variables|Character|GetMesh))
  (Transformation|Teleport (+ (Transformation|GetWorldLocation _mesh) "0, 0,100.000000") (Math|Rotator|MakeRotator 0.0 0.0 (.yaw (Transformation|GetWorldRotation _mesh)))))

(event Input|ActionEvents|InputActionHandbrake
  (params (Key :type Key%20Structure :default "None")))

(event Input|ActionEvents|InputActionJump
  (params (Key :type Key%20Structure :default "None"))
  (:Pressed
    (if (< (Math|Vector|VectorLength (Transformation|GetVelocity)) 2e+01)
      (CallFunction|UprightVehicle))))

(event Input|AxisEvents|InputAxisMoveForward
  (params (AxisValue :type Float%20%28single-precision%29))
  (Class|WheeledVehicleMovementComponent|SetThrottleInput (Variables|Default|GetVehicleMovement) AxisValue))

(event Input|AxisEvents|InputAxisMoveRight
  (params (AxisValue :type Float%20%28single-precision%29))
  (Class|WheeledVehicleMovementComponent|SetSteeringInput (Variables|Default|GetVehicleMovement) AxisValue))

(event Input|AxisEvents|InputAxisLookUp
  (params (AxisValue :type Float%20%28single-precision%29))
  (Pawn|Input|AddControllerPitchInput AxisValue))

(event Input|AxisEvents|InputAxisLookRight
  (params (AxisValue :type Float%20%28single-precision%29))
  (Pawn|Input|AddControllerYawInput AxisValue))

(fn ConstructionScript
  (Development|SetHiddeninGame (Variables|Default|Getsunny) true false))