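; BP_24x24_Parcell is a child parcel Blueprint for 24x24 lots in the AssetsvilleTown2 town set.
; Its construction script maps the Type category (all, nature, parks, residential, commercial or special) to a Min/Max index range in the ParcellClass array.
; Category ranges are hard-coded, so they depend on array order; only ALL follows the array length.
; It then calls the parent construction script with that range set; the event graph holds no active logic.
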(event EventBeginPlay
  (|CallParentFunction) ; This node is disabled and will not be called.\nDrag off pins to build functionality.
)

(event Collision|EventActorBeginOverlap
  (params (OtherActor :type Actor%20Object%20Reference))
  (|CallParentFunction OtherActor) ; This node is disabled and will not be called.\nDrag off pins to build functionality.
)

(event EventTick
  (params (DeltaSeconds :type Float%20%28single-precision%29))
  (|CallParentFunction DeltaSeconds) ; This node is disabled and will not be called.\nDrag off pins to build functionality.
)

(fn ConstructionScript
  (switch Utilities|FlowControl|Switch|SwitchonE_ParcellTypes (Variables|Default|GetType)
    (:NewEnumerator3
      (Variables|Default|SetMin 0)
      (Variables|Default|SetMax (- (Utilities|Array|Length (Variables|Default|GetParcell%20Class)) 1)))
    (:NewEnumerator0
      (Variables|Default|SetMin 0)
      (Variables|Default|SetMax 7))
    (:NewEnumerator4
      (Variables|Default|SetMin 8)
      (Variables|Default|SetMax 13))
    (:NewEnumerator1
      (Variables|Default|SetMin 14)
      (Variables|Default|SetMax 35))
    (:NewEnumerator5
      (Variables|Default|SetMin 36)
      (Variables|Default|SetMax 49))
    (:NewEnumerator6
      (Variables|Default|SetMin 50)
      (Variables|Default|SetMax 51)))
  (|CallParentFunction))