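; BP_48x48_Parcell is a child parcel Blueprint for the 48x48 set in the AssetsvilleTown2 town kit.
; Its construction script maps the Type category to a Min/Max index range in the ParcellClass array, then runs the parent construction script.
; ALL spans the whole array, Commercial and Special get separate ranges, and Nature, Parks and Residental all collapse to the first entry.
; The event graph holds only disabled stubs.
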(event EventBeginPlay
  (|CallParentFunction) ; This node is disabled and will not be called.\nDrag off pins to build functionality.
)

(event Collision|EventActorBeginOverlap
  (params (OtherActor :type Actor%20Object%20Reference))
  (|CallParentFunction OtherActor) ; This node is disabled and will not be called.\nDrag off pins to build functionality.
)

(event EventTick
  (params (DeltaSeconds :type Float%20%28single-precision%29))
  (|CallParentFunction DeltaSeconds) ; This node is disabled and will not be called.\nDrag off pins to build functionality.
)

(fn ConstructionScript
  (switch Utilities|FlowControl|Switch|SwitchonE_ParcellTypes (Variables|Default|GetType)
    (:NewEnumerator3
      (Variables|Default|SetMin 0)
      (Variables|Default|SetMax (- (Utilities|Array|Length (Variables|Default|GetParcell%20Class)) 1)))
    (:NewEnumerator0
      (Variables|Default|SetMin 0)
      (Variables|Default|SetMax 0))
    (:NewEnumerator4
      (Variables|Default|SetMin 0)
      (Variables|Default|SetMax 0))
    (:NewEnumerator1
      (Variables|Default|SetMin 0)
      (Variables|Default|SetMax 0))
    (:NewEnumerator5
      (Variables|Default|SetMin 0)
      (Variables|Default|SetMax 10))
    (:NewEnumerator6
      (Variables|Default|SetMin 11)
      (Variables|Default|SetMax 23)))
  (|CallParentFunction))