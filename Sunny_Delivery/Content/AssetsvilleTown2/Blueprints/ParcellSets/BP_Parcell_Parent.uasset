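; Parent Blueprint for town parcels that spawns one parcel variant through a Child Actor component.
; The Construction Script optionally rolls a random ParcellType between Min and Max, sets the child class from the ParcellClass array at that index, and resets Refresh.
; SaveSelection turns off Randomize to lock the current pick and prints a confirmation, while TryAgain has an empty body.
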(event Custom|Save%20Selection
  (Variables|Default|SetRandomize false)
  (Development|PrintString "Selection Saved"))

(event Custom|TryAgain)

(event EventBeginPlay)

(event Collision|EventActorBeginOverlap
  (params (OtherActor :type Actor%20Object%20Reference)))

(event EventTick
  (params (DeltaSeconds :type Float%20%28single-precision%29)))

(fn ConstructionScript
  (if (Variables|Default|GetRandomize)
    (Variables|Default|SetParcell%20Type (Math|Random|RandomIntegerinRange (Variables|Default|GetMin) (Variables|Default|GetMax))))
  (ChildActorComponent|SetChildActorClass (Variables|Default|GetChildActor) (Utilities|Array|Get(acopy) (Variables|Default|GetParcell%20Class) (Variables|Default|GetParcell%20Type)))
  (Variables|Default|SetRefresh false))