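; BP_Electricity_Pole is a construction-script tool that lays out electricity poles with hanging cables along a spline.
; It adds a mesh at each spline point, then links every socket name to the same socket on the next pole.
; Each cable gets a temporary-shape spline with a tension-lowered midpoint, whose end tangents bend one spline mesh into a sag.
; Flags can remove the first or all poles afterwards, leaving cables intact.
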(event EventBeginPlay)

(event Collision|EventActorBeginOverlap
  (params (OtherActor :type Actor%20Object%20Reference)))

(event EventTick
  (params (DeltaSeconds :type Float%20%28single-precision%29)))

(fn ConstructionScript
  (bind _spline (Variables|Default|GetSpline))
  (bind _poles (Variables|Default|GetPoles))
  (bind _spline_2 (Variables|Default|GetSpline))
  (bind _returnvalue (Spline|GetNumberOfSplinePoints _spline))
  (bind _output (Utilities|Array|Get(acopy) _poles))
  (bind _returnvalue_2 (- _returnvalue 1))
  (CallFunction|CreatePoleMeshArray)
  (for _index (range 0 _returnvalue_2)
    (Transformation|AddLocalOffset (Utilities|Array|Get(acopy) (Variables|Default|GetPoles) _index) (Spline|GetLocationatSplinePoint _spline_2 _index "Local") false false)
    (Transformation|AddLocalRotation (Utilities|Array|Get(acopy) (Variables|Default|GetPoles) _index) (Spline|GetRotationatSplinePoint _spline_2 _index "Local") false false))
  (for _index_2 (range 0 (- (Utilities|Array|Length (Variables|Default|GetSocket%20Names)) 1))
    (CallFunction|AttachCableSplinetoSocket (- _returnvalue_2 1) (Utilities|Array|Get(acopy) (Variables|Default|GetSocket%20Names) _index_2)))
  (if (Variables|Default|GetHide%20All%20Poles)
    (for _index_3 (range 0 _returnvalue_2)
      (Components|StaticMesh|SetStaticMesh (Utilities|Array|Get(acopy) _poles _index_3) 0)
      (Components|DestroyComponent (Utilities|Array|Get(acopy) _poles _index_3)))
    (elif (Variables|Default|GetHide%20First%20Pole)
      (Components|StaticMesh|SetStaticMesh _output 0)
      (Components|DestroyComponent _output))))

(fn CreatePoleMeshArray
  (Utilities|Array|Clear (Variables|Default|GetPoles))
  (for _index (range 0 (- (Spline|GetNumberOfSplinePoints (Variables|Default|GetSpline)) 1))
    (bind _returnvalue (AddComponent|AddStaticMeshComponent false))
    (Components|StaticMesh|SetStaticMesh _returnvalue (Variables|Default|GetStatic%20Mesh))
    (Utilities|Array|Add (Variables|Default|GetPoles) _returnvalue))
  (Variables|Default|SetSocket%20Names (Transformation|GetAllSocketNames (Utilities|Array|Get(acopy) (Variables|Default|GetPoles)))))

(fn AttachCableSplinetoSocket
  (params (Index :type Integer) (SocketName :type Name))
  (bind _poles (Variables|Default|GetPoles))
  (for _index (range 0 Index)
    (if (Transformation|DoesSocketExist (Utilities|Array|Get(acopy) _poles _index) SocketName)
      (CallFunction|CreateCableSpline (.Location (Math|Transform|BreakTransform (Transformation|GetSocketTransform (Utilities|Array|Get(acopy) _poles _index) SocketName "RTS_Actor"))) (.Location (Math|Transform|BreakTransform (Transformation|GetSocketTransform (Utilities|Array|Get(acopy) _poles (+ _index 1)) SocketName "RTS_Actor")))))))

(fn CreateCableSpline
  (params (Start%20Location :type Vector) (End%20Location :type Vector))
  (bind (_x _y _z) (Math|Vector|BreakVector End%20Location))
  (bind (_x_2 _y_2) (Math|Vector|BreakVector Start%20Location))
  (bind _cable_thickness (Variables|Default|GetCable%20Thickness))
  (bind _returnvalue (Math|Vector2D|MakeVector2D _cable_thickness _cable_thickness))
  (bind _returnvalue_2 (AddComponent|AddSplineComponent false))
  (for _index (range 0 (Variables|Default|GetCable%20Spline%20Points))
    (if (== _index 0)
      (Spline|SetLocationatSplinePoint _returnvalue_2 _index Start%20Location "Local" true)
      (elif (== _index 2)
        (Spline|AddSplinePointatIndex _returnvalue_2 End%20Location _index "Local" true)
        (else
          (Spline|SetLocationatSplinePoint _returnvalue_2 _index (Math|Vector|MakeVector (+ _x_2 (/ (- _x _x_2) 2.0)) (+ _y_2 (/ (- _y _y_2) 2.0)) (- _z (Variables|Default|GetCable%20Tension))) "Local" true)))))
  (for _index_2 (range 0 0)
    (bind _returnvalue_3 (AddComponent|AddSplineMeshComponent false))
    (SplineMesh|SetForwardAxis _returnvalue_3 "X" true)
    (SplineMesh|SetStartandEnd _returnvalue_3 (Spline|GetLocationatSplinePoint _returnvalue_2 _index_2 "Local") (Spline|GetTangentatSplinePoint _returnvalue_2 _index_2 "Local") (Spline|GetLocationatSplinePoint _returnvalue_2 (+ _index_2 2) "Local") (Spline|GetTangentatSplinePoint _returnvalue_2 (+ _index_2 2) "Local") true :!class /Script/Engine.SplineMeshComponent)
    (SplineMesh|SetStartScale _returnvalue_3 _returnvalue true :!class /Script/Engine.SplineMeshComponent)
    (SplineMesh|SetEndScale _returnvalue_3 _returnvalue true :!class /Script/Engine.SplineMeshComponent)))