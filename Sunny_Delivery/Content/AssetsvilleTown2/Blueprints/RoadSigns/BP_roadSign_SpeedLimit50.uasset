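; BP_roadSign_SpeedLimit50 is a road sign Blueprint that displays a speed limit as text.
; Its construction script writes the SpeedLimit value into the Number text component and scales that text down for limits of three or more digits, up otherwise.
; The event graph holds only disabled placeholder events, so the sign has no runtime logic there.
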(event EventBeginPlay)

(event Collision|EventActorBeginOverlap
  (params (OtherActor :type Actor%20Object%20Reference)))

(event EventTick
  (params (DeltaSeconds :type Float%20%28single-precision%29)))

(fn ConstructionScript
  (bind _number (Variables|Default|GetNumber))
  (bind _speed_limit (Variables|Default|GetSpeed%20Limit))
  (bind _number_2 (Variables|Default|GetNumber))
  (Rendering|Components|TextRender|SetText _number_2 (Utilities|Text|ToText(Integer) _speed_limit))
  (if (>= _speed_limit 100)
    (Rendering|Components|TextRender|SetYScale _number_2 0.9)
    (Rendering|Components|TextRender|SetXScale _number_2 0.9)
    (else
      (Rendering|Components|TextRender|SetYScale _number 1.2)
      (Rendering|Components|TextRender|SetXScale _number 1.2))))