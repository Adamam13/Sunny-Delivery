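; BP_SmallRoadSystem1 is a configurable small road piece with optional pedestrian crossings, ramps and end sidewalk, plus selectable borders and curb colors.
; The Construction Script reads per-feature flags, assigning meshes to some enabled parts and hiding and destroying components for disabled ones.
; Left and right borders take meshes from RoadBorderTypes, then get a white, yellow or red curb material on slot 1.
; The event graph has no active logic.
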(event EventBeginPlay)

(event Collision|EventActorBeginOverlap
  (params (OtherActor :type Actor%20Object%20Reference)))

(event EventTick
  (params (DeltaSeconds :type Float%20%28single-precision%29)))

(fn ConstructionScript
  (bind _pedestriancrossing_a (Variables|Default|GetPedestrianCrossing_A))
  (bind _pedestriancrossing_b (Variables|Default|GetPedestrianCrossing_B))
  (bind _pedestriancrossing_right (Variables|Default|GetPedestrianCrossing_Right))
  (bind _pedestriancrossing_left (Variables|Default|GetPedestrianCrossing_Left))
  (bind _roadendramp (Variables|Default|GetRoadEndRamp))
  (bind _roadborderright (Variables|Default|GetRoadBorderRight))
  (bind _roadborderleft (Variables|Default|GetRoadBorderLeft))
  (bind _rampright (Variables|Default|GetRampRight))
  (bind _rampleft (Variables|Default|GetRampLeft))
  (bind _roadendsidewalk (Variables|Default|GetRoadEndSidewalk))
  (Utilities|FlowControl|Sequence
    (:then_0
      ;[1 1 1] RoadEnd Ramp
      (if (Variables|Main|GetRoadEnd%20Ramp)
        (Components|StaticMesh|SetStaticMesh _roadendramp "/Game/AssetsvilleTown2/Meshes/RoadSystem/SM_RoadBorder_Ramp.SM_RoadBorder_Ramp")
        (else
          (Rendering|SetVisibility _roadendramp false false)
          (Components|DestroyComponent _roadendramp))))
    (:then_1
      ;[1 1 1] Road Crossings
      (Utilities|FlowControl|Sequence
        (:then_0
          (if (not (Variables|Main|GetCrosswalk%20A))
            (Rendering|SetVisibility _pedestriancrossing_a false false)
            (Components|DestroyComponent _pedestriancrossing_a)
            (if (not (Variables|Main|GetCrosswalk%20B)) :!label _label
              (Rendering|SetVisibility _pedestriancrossing_b false false)
              (Components|DestroyComponent _pedestriancrossing_b))))
        (:then_1
          (goto _label))
        (:then_2
          ;[1 1 1] Side Crossings
          (Utilities|FlowControl|Sequence
            (:then_0
              (if (Variables|RightLane|GetCrosswalk%20Right)
                (Components|StaticMesh|SetStaticMesh _pedestriancrossing_right "/Game/AssetsvilleTown2/Meshes/RoadSystem/SM_Road_Crossing.SM_Road_Crossing")
                (else
                  (Rendering|SetVisibility _pedestriancrossing_right false false)
                  (Components|DestroyComponent _pedestriancrossing_right))))
            (:then_1
              (if (Variables|LeftLane|GetCrosswalk%20Left)
                (Components|StaticMesh|SetStaticMesh _pedestriancrossing_left "/Game/AssetsvilleTown2/Meshes/RoadSystem/SM_Road_Crossing.SM_Road_Crossing")
                (else
                  (Rendering|SetVisibility _pedestriancrossing_left false false)
                  (Components|DestroyComponent _pedestriancrossing_left))))))))
    (:then_2
      ;[1 1 1] Road Borders
      (Components|StaticMesh|SetStaticMesh (Variables|Default|GetRoadBorderLeft) (Utilities|Array|Get(acopy) (Variables|Main|GetRoadBorderTypes) (Variables|LeftLane|GetLeft%20Sidewalk)))
      (Components|StaticMesh|SetStaticMesh (Variables|Default|GetRoadBorderRight) (Utilities|Array|Get(acopy) (Variables|Main|GetRoadBorderTypes) (Variables|RightLane|GetRight%20Sidewalk))))
    (:then_3
      ;[1 1 1] Road End Sidewalk
      (if (Variables|Main|GetRoadEnd%20Sidewalk)
        (Components|StaticMesh|SetStaticMesh _roadendsidewalk "/Game/AssetsvilleTown2/Meshes/RoadSystem/SM_SmallRoadBorder_SidewalkEnd.SM_SmallRoadBorder_SidewalkEnd")
        (else
          (Rendering|SetVisibility _roadendsidewalk false false)
          (Components|DestroyComponent _roadendsidewalk))))
    (:then_4
      ;[1 1 1] Curbs Color
      (Utilities|FlowControl|Sequence
        (:then_0
          (switch Utilities|FlowControl|Switch|SwitchonE_RoadCurbsOptions (Variables|RightLane|GetRight%20Curb%20Color)
            (:NewEnumerator0
              (Rendering|Material|SetMaterial _roadborderright 1 "/Game/AssetsvilleTown2/Materials/MI_curbWhite.MI_curbWhite"))
            (:NewEnumerator1
              (Rendering|Material|SetMaterial _roadborderright 1 "/Game/AssetsvilleTown2/Materials/MI_curbYellow.MI_curbYellow"))
            (:NewEnumerator3
              (Rendering|Material|SetMaterial _roadborderright 1 "/Game/AssetsvilleTown2/Materials/MI_curbRed.MI_curbRed"))))
        (:then_1
          (switch Utilities|FlowControl|Switch|SwitchonE_RoadCurbsOptions (Variables|LeftLane|GetLeft%20Curb%20Color)
            (:NewEnumerator0
              (Rendering|Material|SetMaterial _roadborderleft 1 "/Game/AssetsvilleTown2/Materials/MI_curbWhite.MI_curbWhite"))
            (:NewEnumerator1
              (Rendering|Material|SetMaterial _roadborderleft 1 "/Game/AssetsvilleTown2/Materials/MI_curbYellow.MI_curbYellow"))
            (:NewEnumerator3
              (Rendering|Material|SetMaterial _roadborderleft 1 "/Game/AssetsvilleTown2/Materials/MI_curbRed.MI_curbRed"))))))
    (:then_5
      ;[1 1 1] Ramps
      (Utilities|FlowControl|Sequence
        (:then_0
          (if (Variables|RightLane|GetRight%20Ramp)
            (Components|StaticMesh|SetStaticMesh _rampright "/Game/AssetsvilleTown2/Meshes/RoadSystem/SM_RoadBorder_Ramp.SM_RoadBorder_Ramp")
            (else
              (Rendering|SetVisibility _rampright false false)
              (Components|DestroyComponent _rampright))))
        (:then_1
          (if (Variables|LeftLane|GetLeft%20Ramp)
            (Components|StaticMesh|SetStaticMesh _rampleft "/Game/AssetsvilleTown2/Meshes/RoadSystem/SM_RoadBorder_Ramp.SM_RoadBorder_Ramp")
            (else
              (Rendering|SetVisibility _rampleft false false)
              (Components|DestroyComponent _rampleft))))))))