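; BP_CarRandomizer is a placeable vehicle prop that picks a random skeletal mesh in its construction script.
; A CarType setting chooses which mesh list to draw from; standard, sport and truck types also get a random body color on material slot 0, while trailers do not.
; The result is saved to SelectedVehicle and SelectedMaterial, which LockVehicleSelection reapplies instead of rerolling.
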(event EventBeginPlay)

(event Collision|EventActorBeginOverlap
  (params (OtherActor :type Actor%20Object%20Reference)))

(event EventTick
  (params (DeltaSeconds :type Float%20%28single-precision%29)))

(fn ConstructionScript
  (bind _carlist_trucks (Variables|Default|GetCarList_Trucks))
  (bind _carlist_trucktrailers (Variables|Default|GetCarList_TruckTrailers))
  (bind _carlist_smalltrailers (Variables|Default|GetCarList_SmallTrailers))
  (bind _skeletalmesh (Variables|Default|GetSkeletalMesh))
  (bind _carcolors (Variables|Default|GetCarColors))
  (bind _carlist_standard (Variables|Default|GetCarList_Standard))
  (bind _carlist_sport (Variables|Default|GetCarList_Sport))
  (if (Variables|Default|GetLock%20Vehicle%20Selection)
    (Class|SkinnedMeshComponent|SetSkeletalMesh (Variables|Default|GetSkeletalMesh) (Variables|Default|GetSelectedVehicle) true)
    (Rendering|Material|SetMaterial (Variables|Default|GetSkeletalMesh) 0 (Variables|Default|GetSelected%20Material))
    (Variables|Default|SetRefresh false)
    (else
      (switch Utilities|FlowControl|Switch|SwitchonE_VehicleTypes (Variables|Default|GetCarType)
        (:NewEnumerator0
          (Class|SkinnedMeshComponent|SetSkeletalMesh (Variables|Default|GetSkeletalMesh) (Utilities|Array|Get(acopy) _carlist_standard (Math|Random|RandomInteger (Utilities|Array|Length _carlist_standard))) true)
          (Rendering|Material|SetMaterial (Variables|Default|GetSkeletalMesh) 0 (Utilities|Array|Get(acopy) _carcolors (Math|Random|RandomInteger (Utilities|Array|Length _carcolors))) :!label _label))
        (:NewEnumerator1
          (Class|SkinnedMeshComponent|SetSkeletalMesh (Variables|Default|GetSkeletalMesh) (Utilities|Array|Get(acopy) _carlist_sport (Math|Random|RandomInteger (Utilities|Array|Length _carlist_sport))) true)
          (goto _label))
        (:NewEnumerator2
          (Class|SkinnedMeshComponent|SetSkeletalMesh (Variables|Default|GetSkeletalMesh) (Utilities|Array|Get(acopy) _carlist_trucks (Math|Random|RandomInteger (Utilities|Array|Length _carlist_trucks))) true)
          (goto _label))
        (:NewEnumerator3
          (Class|SkinnedMeshComponent|SetSkeletalMesh (Variables|Default|GetSkeletalMesh) (Utilities|Array|Get(acopy) _carlist_trucktrailers (Math|Random|RandomInteger (Utilities|Array|Length _carlist_trucktrailers))) true))
        (:NewEnumerator4
          (Class|SkinnedMeshComponent|SetSkeletalMesh (Variables|Default|GetSkeletalMesh) (Utilities|Array|Get(acopy) _carlist_smalltrailers (Math|Random|RandomInteger (Utilities|Array|Length _carlist_smalltrailers))) true)))
      (Variables|Default|SetRefresh false)
      (Variables|Default|SetSelectedVehicle (Variables|/Script/Engine.SkinnedMeshComponent|GetSkeletalMesh _skeletalmesh))
      (Variables|Default|SetSelected%20Material (Rendering|Material|GetMaterial _skeletalmesh 0)))))